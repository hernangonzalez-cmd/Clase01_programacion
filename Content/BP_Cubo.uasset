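; BP_Cubo is a test cube actor that moves and sets a fixed rotation every frame.
; Tick increments a counter and sets the actor's X location from it at a fixed height, so speed depends on frame rate.
; It also stores DeltaSeconds as text in a variable that nothing here reads.
; BeginPlay, overlap and construction script are empty, and disconnected offset, delay and position-increment nodes never run.
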(event `self.ReceiveBeginPlay`
  ; Se ejecuta al comenzar el juego
)

(event `self.ReceiveTick`
  (params (DeltaSeconds :type "Float (single-precision)"))
  ; se ejecuta un avez por frame
  (set `self.Texto` (`KismetStringLibrary.Conv_DoubleToString` DeltaSeconds))
  (bind _output_get (set `self.Numero` (+ (`self.Numero`) 1)))
  (`self.K2_SetActorLocation` (`KismetMathLibrary.MakeVector` (`KismetMathLibrary.Conv_IntToDouble` _output_get) 0.0 260.0))
  (`self.K2_SetActorRotation` (`KismetMathLibrary.MakeRotator` 1.0 1.0 6.0)))

(fn `UserConstructionScript`)